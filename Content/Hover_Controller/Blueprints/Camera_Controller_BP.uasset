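; Camera controller component that rotates the owning actor's spring arm from yaw and look-up input while active.
; On BeginPlay it builds an array of the owner's spring arms, indexed by numbers in their object names.
; An active-state event seeds pitch and yaw from the selected arm's rotation.
; Look input, scaled by a multiplier with pitch inverted, accumulates into those values, which set and cache the arm's relative rotation.
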(event Custom|Set%20Camera%20Rotation
  (params (New%20Spring%20Arm%20Relative%20Rotation :type Rotator))
  (bind (_roll _pitch _yaw) (Math|Rotator|BreakRotator New%20Spring%20Arm%20Relative%20Rotation))
  ;[1 1 1] Set Cameras Rotation Event
  (Variables|Default|SetCamera%20pitch _pitch)
  (Variables|Default|Setcamera%20yaw _yaw))

(event Custom|Add%20look%20at%20direction%20%28Camera%29
  (params (Yaw%20input :type Float%20%28single-precision%29) (Look%20up%20input :type Float%20%28single-precision%29))
  (bind _spring_arm__ (Variables|Camera/RotationControls|GetSpring%20Arm%20#))
  (bind _camera_multiplier (Variables|Camera/RotationControls|GetCamera%20Multiplier))
  (bind _spring_arm (Variables|Default|GetSpring%20Arm))
  (bind _output (Utilities|Array|Get(acopy) _spring_arm _spring_arm__))
  ;[1 1 1] Set spring arm rotation
  ;;[1 1 1] Save Inputs
  (if (Variables|Default|GetController%20Active)
    (Variables|Default|SetYaw%20input Yaw%20input)
    (Variables|Default|SetLook%20up%20input Look%20up%20input)
    ;;[1 1 1] Make Changes To Saved Pitch And Yaw Variables With New Changes
    (bind _output_get (Variables|Default|SetCamera%20pitch (+ (Variables|Default|GetCamera%20pitch) (* (* (Variables|Default|GetLook%20up%20input) -1.0) _camera_multiplier))))
    (bind _output_get_2 (Variables|Default|Setcamera%20yaw (+ (Variables|Default|Getcamera%20yaw) (* _camera_multiplier (Variables|Default|GetYaw%20input)))))
    ;;[1 1 1] Rotate Camera
    (Transformation|SetRelativeRotation _output (Math|Rotator|MakeRotator 0.0 _output_get _output_get_2) false false)
    (Variables|Camera/RotationControls|SetCached%20Camera%20Rotation (Variables|/Script/Engine.SceneComponent|GetRelativeRotation _output))))

(event Custom|Is%20Active%20%28Camera%29
  (params (Controller%20Active :type Boolean))
  (bind _spring_arm__ (Variables|Camera/RotationControls|GetSpring%20Arm%20#))
  (bind _spring_arm (Variables|Default|GetSpring%20Arm))
  (bind _output (Utilities|Array|Get(acopy) _spring_arm _spring_arm__))
  (bind _relativerotation (Variables|/Script/Engine.SceneComponent|GetRelativeRotation _output))
  ;[1 1 1] Set variables when active
  (Variables|Default|SetController%20Active Controller%20Active)
  (if (Variables|Default|GetController%20Active)
    ;;[1 1 1] Update Camera Rotation
    (Variables|Default|SetCamera%20pitch (.pitch _relativerotation))
    (Variables|Default|Setcamera%20yaw (.yaw _relativerotation))))

(event EventBeginPlay
  (bind _returnvalue (Components|GetOwner))
  (bind _spring_arm__ (Variables|Camera/RotationControls|GetSpring%20Arm%20#))
  (bind _spring_arm (Variables|Default|GetSpring%20Arm))
  (bind _returnvalue_2 (Actor|GetComponentsByClass _returnvalue "/Script/Engine.SpringArmComponent"))
  (bind _output (Utilities|Array|Get(acopy) _spring_arm _spring_arm__))
  (bind _relativerotation (Variables|/Script/Engine.SceneComponent|GetRelativeRotation _output))
  ;[1 1 1] Create Array Of Spring Arms With Numbers In Their Name (number can go up to total number of spring arms)
  (for _array_element _returnvalue_2
    (for (_ _array_index) _returnvalue_2
      (if (Utilities|String|Contains (Utilities|GetObjectName _array_element) (Utilities|String|ToString(Integer) _array_index))
        (Utilities|Array|SetArrayElem (Variables|Default|GetSpring%20Arm) _array_index _array_element true))))
  ;[1 1 1] Set variables when active
  (if (Variables|Default|GetController%20Active)
    ;;[1 1 1] Update Camera Rotation
    (Variables|Default|SetCamera%20pitch (.pitch _relativerotation))
    (Variables|Default|Setcamera%20yaw (.yaw _relativerotation))))